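; Troll enemy Blueprint that overrides the hit reaction and attaches its weapon to the mesh's Smash socket at construction.
; While alive, it plays the sound mapped to the attacking weapon.
; If such a sound exists and the hit type is not Still, it turns to face opposite the hit direction and plays a hit montage, choosing the starting section by hit type.
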(event `self.Hit`
  (bind _hittype (`BaseDamageType.HitType` (`self.HitDamageType`)))
  (bind (_returnvalue_roll _returnvalue_pitch _returnvalue_yaw) (`KismetMathLibrary.BreakRotator` (`KismetMathLibrary.Conv_VectorToRotator` (`KismetMathLibrary.NegateVector` (`self.HitDirection`)))))
  (bind (_value _returnvalue) (`BlueprintMapLibrary.Map_Find` (`self.HitSound`) (`BaseDamageType.HitWeapon` (`self.HitDamageType`))))
  ;[1 1 1] Override hit function for troll
  (if (`self.IsAlive`)
    (if _returnvalue
      (`GameplayStatics.PlaySoundAtLocation` _value (`self.K2_GetActorLocation`) (struct) 1.0 1.0 0.0 null null null)
      (if (`|EnumInequality` _hittype "EDT_Still")
        (bind _hitmontage (`self.HitMontage`)
          (:`then`
            (`self.K2_SetActorRotation` (`KismetMathLibrary.MakeRotator` 0.0 0.0 _returnvalue_yaw))
            (`|PlayMontage` (`self.Mesh`) _hitmontage 1.0 0.0 (select `EHitDamageType` _hittype :`EDT_Front` "Hit" :`EDT_Left` "Hit" :`EDT_Right` "Hit" :`EDT_Heavy` "Heavy" :`EDT_ToBack` "HitToBack" :`EDT_Still` "None" :!type "Name")))
          (:`else`))))))

(fn `UserConstructionScript`
  (`SceneComponent.K2_AttachToComponent` (`self.Weapon`) (`self.Mesh`) "Smash" "SnapToTarget" "SnapToTarget" "KeepRelative" true))