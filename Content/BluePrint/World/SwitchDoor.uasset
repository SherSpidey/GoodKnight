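; SwitchDoor is an interactable switch that opens and closes a door.
; Beginning interaction plays a timeline that moves the switch along Z from its initial location, and ending interaction reverses it.
; Beginning interaction also checks an Open flag, plays the matching door sound, and plays or reverses a second timeline that yaws the door from its initial rotation.
; The flag toggles when that timeline finishes.
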(event `self.EndInteract`
  (bind (_initialswitchlocation_x _initialswitchlocation_y _initialswitchlocation_z) (`KismetMathLibrary.BreakVector` (`self.InitialSwitchLocation`)))
  (bind (_direction _location) (`Timeline|InteractSwitch` :!via `Reverse` :!label _label)
    (:`Update`
      (`SceneComponent.K2_SetWorldLocation` (`self.InteractObject`) (`KismetMathLibrary.MakeVector` _initialswitchlocation_x _initialswitchlocation_y (+ _initialswitchlocation_z _location)) false false))))

(event `self.BeginInteract`
  (bind (_initialobjectrotation_roll _initialobjectrotation_pitch _initialobjectrotation_yaw) (`KismetMathLibrary.BreakRotator` (`self.InitialObjectRotation`)))
  (`|ExecutionSequence`
    (:`then_0`
      (goto _label))
    (:`then_1`
      (if (not (`self.Open`))
        (`GameplayStatics.PlaySoundAtLocation` "/Game/Asset/Audio/SFX/Player/Cue/DoorOpen_Cue.DoorOpen_Cue" (`self.InitialObjectLocation`) (struct) 1.0 1.0 0.0 null null null)
        (bind (_direction _rotate) (`Timeline|InteractTarget` :!label _label_2)
          (:`Update`
            (`SceneComponent.K2_SetWorldRotation` (`self.RespondObject`) (`KismetMathLibrary.MakeRotator` _initialobjectrotation_roll _initialobjectrotation_pitch (+ _initialobjectrotation_yaw _rotate)) false false))
          (:`Finished`
            (set `self.Open` (not (`self.Open`)))))
        (else
          (`GameplayStatics.PlaySoundAtLocation` "/Game/Asset/Audio/SFX/Player/Cue/DoorClose_Cue.DoorClose_Cue" (`self.InitialObjectLocation`) (struct) 1.0 1.0 0.0 null null null)
          (goto _label_2 :!via `Reverse`))))))

(fn `UserConstructionScript`)